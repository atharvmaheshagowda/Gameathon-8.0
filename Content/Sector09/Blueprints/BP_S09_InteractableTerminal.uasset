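; Sector 09 interactable terminal that grants a one-time, classified memory archive access message when the player presses E in range.
; Overlapping the InteractionBox sets CanInteract and shows an interaction prompt widget, removed on end overlap, with no check on which actor overlaps.
; The first E press while in range sets IsActivated and displays the message via PrintString.
; The terminal message widget nodes are unconnected and never run.
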(event OnComponentBeginOverlap(InteractionBox)
  (params (OverlappedComponent :type Primitive%20Component%20Object%20Reference) (OtherActor :type Actor%20Object%20Reference) (OtherComp :type Primitive%20Component%20Object%20Reference) (OtherBodyIndex :type Integer) (bFromSweep :type Boolean) (SweepResult :type Hit%20Result%20Structure%20%28by%20ref%29))
  (Variables|Default|SetCanInteract true)
  (bind _returnvalue (UserInterface|CreateWidget "/Game/Sector09/UI/WBP_S09_InteractionPrompt.WBP_S09_InteractionPrompt_C"))
  (bind _output_get (Variables|Default|SetInteractionPromptRef _returnvalue))
  (UserInterface|Viewport|AddtoViewport _output_get 0))

(event OnComponentEndOverlap(InteractionBox)
  (params (OverlappedComponent :type Primitive%20Component%20Object%20Reference) (OtherActor :type Actor%20Object%20Reference) (OtherComp :type Primitive%20Component%20Object%20Reference) (OtherBodyIndex :type Integer))
  (Variables|Default|SetCanInteract false)
  (Widget|RemovefromParent (Variables|Default|GetInteractionPromptRef)))

(event EventBeginPlay)

(event Collision|EventActorBeginOverlap
  (params (OtherActor :type Actor%20Object%20Reference)))

(event EventTick
  (params (DeltaSeconds :type Float%20%28single-precision%29)))

(event Input|KeyboardEvents|E
  (params (Key :type Key%20Structure :default "None"))
  (:Pressed
    (if (Variables|Default|GetCanInteract)
      (if (not (Variables|Default|GetIsActivated))
        (Variables|Default|SetIsActivated true)
        (Development|PrintString "CLASSIFIED // SECTOR 09 
MEMORY ARCHIVE ACCESS GRANTED 
DATA RECOVERY PROTOCOL INITIALIZED")))))

(fn ConstructionScript)